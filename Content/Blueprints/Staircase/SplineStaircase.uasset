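; Spline staircase actor whose construction script derives the sizing values for a run of stairs, optionally several steps wide.
; Step count comes from a target height or fixed count, then sets grid extents before and after the parent construction script runs.
; The scale multiplier is immediately overwritten by the clamp on raw stair extents.
; Vertical bounds height is overridden using spline length, while min/max bounds defer to the parent.
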(event EventBeginPlay
  (|CallParentFunction) ; This node is disabled and will not be called.\nDrag off pins to build functionality.
)

(event Collision|EventActorBeginOverlap
  (params (OtherActor :type Actor%20Object%20Reference))
  (|CallParentFunction OtherActor) ; This node is disabled and will not be called.\nDrag off pins to build functionality.
)

(event EventTick
  (params (DeltaSeconds :type Float%20%28single-precision%29))
  (|CallParentFunction DeltaSeconds) ; This node is disabled and will not be called.\nDrag off pins to build functionality.
)

(fn ConstructionScript
  (bind _stairextents (Variables|01-Stairs|GetStairExtents))
  (Utilities|FlowControl|Sequence
    (:then_0
      (Variables|PCGINTERNAL|SetGEN_StairExtents (* (Variables|01-Stairs|GetStairExtents) (Variables|01-Stairs|GetStairScaleMultiplier))))
    (:then_1
      (Variables|PCGINTERNAL|SetGEN_StairExtents (Math|Vector|MakeVector (Math|Float|Max(Float) (.x _stairextents) 1.0) (Math|Float|Max(Float) (.y _stairextents) 1.0) (Math|Float|Max(Float) (.z _stairextents) 1.0))))
    (:then_2
      (if (Variables|PCGINTERNAL|GetUseTargetHeight)
        (Variables|PCGINTERNAL|SetGEN_Count (Math|Float|Ceil (/ (Variables|PCGINTERNAL|GetTargetHeight) (.z (Variables|PCGINTERNAL|GetGEN_StairExtents)))))
        (else
          (Variables|PCGINTERNAL|SetGEN_Count (Variables|PCGINTERNAL|GetStairCount)))))
    (:then_3
      (bind _output_get (Variables|PCGINTERNAL|SetGEN_UseHorizontalGrid (> (Variables|01-Stairs|GetHorizontalCount) 1)))
      (if _output_get
        (Variables|PCGINTERNAL|SetGEN_StairHorizontalGridExtents (Math|Vector|MakeVector (+ (.x (Variables|PCGINTERNAL|GetGEN_StairExtents)) 1.0) (* (.y (Variables|PCGINTERNAL|GetGEN_StairExtents)) (Variables|01-Stairs|GetHorizontalCount)) (+ (.z (Variables|PCGINTERNAL|GetGEN_StairExtents)) 1.0)))))
    (:then_4
      (|CallParentFunction))
    (:then_5
      (Variables|PCGINTERNAL|SetGEN_StairGridExtent (Math|Vector|MakeVector (* (.x (Variables|PCGINTERNAL|GetGEN_StairExtents)) (Variables|PCGINTERNAL|GetGEN_Count)) (.y (Variables|PCGINTERNAL|GetGEN_StairExtents)) (.z (Variables|PCGINTERNAL|GetGEN_StairExtents)))))))

(fn GetBoundsMinMax
  (bind (_min _max) (|CallParentFunction))
  (return _min _max))

(fn GetBoundsVerticalHeight
  (bind _spline (Variables|Default|GetSpline))
  (bind _stairextents (Variables|01-Stairs|GetStairExtents))
  (bind (_x _y _z) (Math|Vector|BreakVector _stairextents))
  (bind _returnvalue (Spline|GetSplineLength _spline))
  (bind _returnvalue_2 (/ _returnvalue _x))
  (return (.Z (Math|Vector|BreakVector (Math|Vector|MakeVector (* (Variables|PCGINTERNAL|GetGEN_Count) _returnvalue_2) (* _y (Variables|01-Stairs|GetHorizontalCount)) (/ (* _z _returnvalue_2) 2.0))))))