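; Staircase Blueprint that derives the dimensions and step count for a generated staircase, with no active runtime event logic.
; The construction script scales and clamps step extents, takes the count directly or from a target height, and sizes an optional horizontal grid.
; It calls the parent construction script before setting the stair grid extent.
; GetBoundsMinMax returns bounds spanning all steps and columns, starting at the origin in X and Z and centered in Y.
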(event EventBeginPlay
  (|CallParentFunction) ; This node is disabled and will not be called.\nDrag off pins to build functionality.
)

(event Collision|EventActorBeginOverlap
  (params (OtherActor :type Actor%20Object%20Reference))
  (|CallParentFunction OtherActor) ; This node is disabled and will not be called.\nDrag off pins to build functionality.
)

(event EventTick
  (params (DeltaSeconds :type Float%20%28single-precision%29))
  (|CallParentFunction DeltaSeconds) ; This node is disabled and will not be called.\nDrag off pins to build functionality.
)

(fn ConstructionScript
  (Utilities|FlowControl|Sequence
    (:then_0
      (Variables|PCGINTERNAL|SetGEN_StairExtents (* (Variables|01-Stairs|Size|GetStairExtents) (Variables|01-Stairs|GetStairScaleMultiplier))))
    (:then_1
      (Variables|PCGINTERNAL|SetGEN_StairExtents (Math|Vector|MakeVector (Math|Float|Max(Float) (.x (Variables|PCGINTERNAL|GetGEN_StairExtents)) 1.0) (Math|Float|Max(Float) (.y (Variables|PCGINTERNAL|GetGEN_StairExtents)) 1.0) (Math|Float|Max(Float) (.z (Variables|PCGINTERNAL|GetGEN_StairExtents)) 1.0))))
    (:then_2
      (if (Variables|01-Stairs|Size|GetUseTargetHeight)
        (Variables|PCGINTERNAL|SetGEN_Count (Math|Float|Ceil (/ (Variables|01-Stairs|Size|GetTargetHeight) (.z (Variables|PCGINTERNAL|GetGEN_StairExtents)))))
        (else
          (Variables|PCGINTERNAL|SetGEN_Count (Variables|01-Stairs|Size|GetStairCount)))))
    (:then_3
      (bind _output_get (Variables|PCGINTERNAL|SetGEN_UseHorizontalGrid (> (Variables|01-Stairs|Size|GetHorizontalCount) 1)))
      (if _output_get
        (Variables|PCGINTERNAL|SetGEN_StairHorizontalGridExtents (Math|Vector|MakeVector (+ (.x (Variables|PCGINTERNAL|GetGEN_StairExtents)) 1.0) (* (.y (Variables|PCGINTERNAL|GetGEN_StairExtents)) (Variables|01-Stairs|Size|GetHorizontalCount)) (+ (.z (Variables|PCGINTERNAL|GetGEN_StairExtents)) 1.0)))))
    (:then_4
      (|CallParentFunction))
    (:then_5
      (Variables|PCGINTERNAL|SetGEN_StairGridExtent (Math|Vector|MakeVector (* (.x (Variables|PCGINTERNAL|GetGEN_StairExtents)) (Variables|PCGINTERNAL|GetGEN_Count)) (.y (Variables|PCGINTERNAL|GetGEN_StairExtents)) (.z (Variables|PCGINTERNAL|GetGEN_StairExtents)))))))

(fn GetBoundsMinMax
  (bind _gen_stairextents (Variables|PCGINTERNAL|GetGEN_StairExtents))
  (bind _gen_count (Variables|PCGINTERNAL|GetGEN_Count))
  (bind _horizontalcount (Variables|01-Stairs|Size|GetHorizontalCount))
  (bind (_x _y _z) (Math|Vector|BreakVector _gen_stairextents))
  (bind _returnvalue (* _z _gen_count))
  (bind _returnvalue_2 (* _gen_count _x))
  (bind _returnvalue_3 (* _y _horizontalcount))
  (bind _returnvalue_4 (Math|Vector|MakeVector _returnvalue_2 _returnvalue_3 _returnvalue))
  (bind _returnvalue_5 (* _returnvalue_4 "1.000000,0.000000,0.000000"))
  (|CallParentFunction)
  (return (+ (* _returnvalue_4 "-1.000000,-1.000000,0.000000") _returnvalue_5) (+ (* _returnvalue_4 "1.000000,1.000000,1.000000") _returnvalue_5)))