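; BuildingSpline is a spline actor that generates modular buildings through PCG from a base recipe, with optional top and bottom recipes.
; The construction script resolves settings into GEN variables for footprint, floors, walls, corners and offset, and flattens spline point heights.
; It groups slots with non-default pipelines into per-pipeline bitmasks.
; Helper functions recenter the origin, flip the spline, regenerate PCG and print instance counts.
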(event EventBeginPlay
  (|CallParentFunction) ; This node is disabled and will not be called.\nDrag off pins to build functionality.
)

(event Collision|EventActorBeginOverlap
  (params (OtherActor :type Actor%20Object%20Reference))
  (|CallParentFunction OtherActor) ; This node is disabled and will not be called.\nDrag off pins to build functionality.
)

(event EventTick
  (params (DeltaSeconds :type Float%20%28single-precision%29))
  (|CallParentFunction DeltaSeconds) ; This node is disabled and will not be called.\nDrag off pins to build functionality.
)

(fn ConstructionScript
  (bind _footprint (Properties|GetFootprintSize))
  (bind _buildingoffset (Variables|00-Core|GetBuildingOffset))
  (bind _building_z_count (Variables|00-Core|GetBuilding%20Z%20Count))
  (bind _baserecipe (Variables|01-Recipes|GetBaseRecipe))
  (|CallParentFunction)
  (Utilities|FlowControl|Sequence
    (:then_0
      (Variables|01-Recipes|GetBaseRecipe
        (:then
          (Variables|PCGINTERNAL|SetGEN_Enabled_0 true)
          (Utilities|FlowControl|Sequence
            (:then_0
              ;[0.3628 0.3628 0.3628 0.5] Extract
              (Variables|PCGINTERNAL|SetGEN_FootprintSize (Math|Vector|SelectVector (* (.z (Transformation|GetActorScale3D)) _footprint) _footprint (Utilities|Enum|Equal(Enum) (Variables|00-Core|Editor|GetVerticalScalingBehavior) "NewEnumerator1")))
              ;[0.3628 0.3628 0.3628 0.5] Extract Z Count
              (Variables|PCGINTERNAL|SetGEN_ZCount (Math|Integer|Max(Integer) (Math|Integer|SelectInt (Math|Float|Round (* (.z (Transformation|GetActorScale3D)) _building_z_count)) _building_z_count (Utilities|Enum|Equal(Enum) (Variables|00-Core|Editor|GetVerticalScalingBehavior) "NewEnumerator2")) 1)))))
        (:else
          (Variables|PCGINTERNAL|SetGEN_Enabled_0 false))))
    (:then_1
      (if (Variables|PCGINTERNAL|GetGEN_Enabled_0)
        (Utilities|FlowControl|Sequence
          (:then_0
            ;[0.3628 0.3628 0.3628 0.176] Extract High Level Booleans
            (Utilities|FlowControl|Sequence
              (:then_0
                ;;[0.3628 0.3628 0.3628 0.5] Walls
                (Variables|PCGINTERNAL|SetGEN_WallsEnabled (Variables|02-Walls|GetSpawnWalls)))
              (:then_1
                ;;[0.3628 0.3628 0.3628 0.5] Floors
                (if (Variables|Default|GetIsClosedLoop)
                  (Variables|PCGINTERNAL|SetGEN_FloorsEnabled (Variables|03-Floors|GetSpawnFloors))
                  (Variables|PCGINTERNAL|SetGEN_CeilingEnabled (Variables|03-Floors|GetSpawnCeiling))
                  (else
                    (Variables|PCGINTERNAL|SetGEN_FloorsEnabled false)
                    (Variables|PCGINTERNAL|SetGEN_CeilingEnabled false))))
              (:then_2
                ;;[0.125 0.125 0.125 0.5] Corners
                (Utilities|FlowControl|Sequence
                  (:then_0
                    (bind _output_get (Variables|PCGINTERNAL|SetGEN_InCornerMode_Walls (select (Variables|02-Walls|Corners|GetDisableCornersIn) "NewEnumerator0" (Variables|/ArchitectCore/Core/ArchitectAssets/ArchitectFullRecipe.ArchitectFullRecipe_C|GetInvertedCornerMode _baserecipe))))
                    (bind _output_get_2 (Variables|PCGINTERNAL|SetGEN_OutCornerMode_Walls (select (Variables|02-Walls|Corners|GetDisableCornersOut) "NewEnumerator0" (Variables|/ArchitectCore/Core/ArchitectAssets/ArchitectFullRecipe.ArchitectFullRecipe_C|GetOutsideCornerMode _baserecipe))))
                    (Variables|PCGINTERNAL|SetGEN_CornersEnabled (not (and (Utilities|Enum|Equal(Enum) _output_get "NewEnumerator0") (Utilities|Enum|Equal(Enum) _output_get_2 "NewEnumerator0")))))))))
          (:then_1
            ;[0.3628 0.3628 0.3628 0.5] May do some processing on floors, to remove duplicates or clamp to bounds
            (if (Variables|03-Floors|Multifloor|GetEnableMultifloor)
              (Variables|PCGINTERNAL|SetGEN_MultiFloors (Variables|03-Floors|Multifloor|GetMulti%20Floors))
              (Variables|PCGINTERNAL|SetGEN_MultifloorEnabled (Variables|03-Floors|Multifloor|GetEnableMultifloor))
              (Variables|PCGINTERNAL|SetGEN_SpawnGroundFloor (Variables|03-Floors|GetSpawnGroundFloor))
              (else
                (Variables|PCGINTERNAL|SetGEN_MultifloorEnabled false))))
          (:then_3
            ;[1 1 1] Top Bottom Recipes
            (Utilities|FlowControl|Sequence
              (:then_0
                (Variables|01-Recipes|GetTopRecipe
                  (:then
                    (Variables|PCGINTERNAL|SetGEN_OverrideTop (Variables|01-Recipes|GetEnableTopRecipe)))
                  (:else
                    (Variables|PCGINTERNAL|SetGEN_OverrideTop false))))
              (:then_1
                (Variables|01-Recipes|GetBottomRecipe
                  (:then
                    (Variables|PCGINTERNAL|SetGEN_OverrideBottom (Variables|01-Recipes|GetEnableBottomRecipe)))
                  (:else
                    (Variables|PCGINTERNAL|SetGEN_OverrideBottom false))))))
          (:then_4
            (CallFunction|SnapPointsZ))
          (:then_5
            ;[1 1 1] Calculate Absolute Offset
            (bind _output_get_3 (Variables|PCGINTERNAL|SetGEN_BuildingOffset (* (Math|Transform|TransformDirection (Transformation|GetActorTransform) (Math|Vector|Normalize _buildingoffset)) (Math|Vector|VectorLength _buildingoffset))))
            (Variables|PCGINTERNAL|SetGEN_HasBuildingOffset (Utilities|Operators|NotEqual(!=) :A _output_get_3)))
          (:then_6
            ;[1 1 1] Pipelines
            (Utilities|FlowControl|Sequence
              (:then_0
                (Utilities|IsValid (Variables|01-Recipes|GetOverridePipeline)
                  (:Is%20Valid
                    (Variables|PCGINTERNAL|SetGEN_UseInstanceOverride false))
                  (:Is%20Not%20Valid
                    (Variables|PCGINTERNAL|SetGEN_UseInstanceOverride false))))
              (:then_1
                (bind (_has_asset_overrides _has_pipeline_overrides _override_pipelines _override_target_masks) (PCGINTERNAL|SearchforOverrides))
                (Variables|PCGINTERNAL|SetGEN_HasAssetOverrides _has_asset_overrides)
                (Variables|PCGINTERNAL|SetGEN_HasPipelineOverrides _has_pipeline_overrides)
                (Variables|PCGINTERNAL|SetGEN_Pipelines _override_pipelines)
                (Variables|PCGINTERNAL|SetGEN_PipelineTargets _override_target_masks)))))))))

(fn GetBoundsVerticalHeight
  (return (* (.z (Properties|GetFootprintSize)) (Variables|00-Core|GetBuilding%20Z%20Count))))

(fn GetFootprintSize
  (bind _baserecipe (Variables|01-Recipes|GetBaseRecipe)
    (:then
      (if (> (Math|Vector|VectorLength (Variables|/ArchitectCore/Core/ArchitectAssets/ArchitectFullRecipe.ArchitectFullRecipe_C|GetFootprint _baserecipe)) 3.0)
        _
        (else
          (CallFunction|PrintErrorwithInfo "Given Recipe with very small footprint, make this larger or it could spawn a huge number of objects" true)))
      (return (* (Variables|00-Core|GetFootprintScaleMultiplier) (Variables|/ArchitectCore/Core/ArchitectAssets/ArchitectFullRecipe.ArchitectFullRecipe_C|GetFootprint _baserecipe))))
    (:else
      (CallFunction|PrintErrorwithInfo "Missing Base Recipe" false)
      (return "50.000000,50.000000,50.000000"))))

(fn ResetOrigintoBuilding
  (bind _spline (Variables|Default|GetSpline))
  (bind _returnvalue (Spline|GetSplinePointAt _spline 0 "Local"))
  (bind _position (Utilities|Struct|BreakSplinePoint _returnvalue))
  (bind _returnvalue_2 (* _position -1.0))
  (Utilities|FlowControl|Sequence
    (:then_0
      (Transformation|SetRelativeLocation (Variables|Default|GetSpline) "0, 0, 0" false false)
      (LocalVariables|SetLS%20Offset (Math|Vector|MakeVector (.x _returnvalue_2) (.y _returnvalue_2) 0.0))
      (LocalVariables|SetLS%20Z 0.0)
      (for _index (range 0 (- (Spline|GetNumberOfSplinePoints (Variables|Default|GetSpline)) 1))
        (Spline|SetLocationatSplinePoint (Variables|Default|GetSpline) _index (Math|Vector|MakeVector (.x (+ (Spline|GetLocationatSplinePoint (Variables|Default|GetSpline) _index "Local") (LocalVariables|GetLS%20Offset))) (.y (+ (Spline|GetLocationatSplinePoint (Variables|Default|GetSpline) _index "Local") (LocalVariables|GetLS%20Offset))) (LocalVariables|GetLS%20Z)) "Local" false))
      (Transformation|SetActorLocation (+ (* (LocalVariables|GetLS%20Offset) -1.0) (Transformation|GetActorLocation)) false false)
      (Spline|UpdateSpline (Variables|Default|GetSpline))
      (CallFunction|UpdateBoundsforPCG))
    (:then_1
      (PCG|Generate (Variables|Default|GetPCG_Main) true))))

(fn RefreshGeneration
  (Class|PCGComponent|GenerateLocal (Variables|Default|GetPCG_Main) true))

(fn SearchforOverrides
  (bind _pipelines (LocalVariables|Getpipelines))
  (bind _baserecipe (Variables|01-Recipes|GetBaseRecipe))
  (bind _pipelines_2 (LocalVariables|Getpipelines))
  (bind _pipelines_3 (LocalVariables|Getpipelines))
  (Variables|01-Recipes|GetBaseRecipe
    (:then
      (Utilities|FlowControl|Sequence
        (:then_0
          (bind _slot_lookups (Default|GetSlotsasLookup _baserecipe))
          (bind _values (Utilities|Map|Values _slot_lookups))
          (for _array_element _values
            (if (.Enabled (Utilities|Struct|BreakS_ArchitectSlot _array_element))
              (if (!= (.Pipeline (Utilities|Struct|BreakS_ArchitectSlot _array_element)) (Variables|/ArchitectCore/Core/ArchitectAssets/ArchitectFullRecipe.ArchitectFullRecipe_C|GetDefaultPipeline _baserecipe))
                (if (Utilities|Map|Contains _pipelines_3 (.Pipeline (Utilities|Struct|BreakS_ArchitectSlot _array_element)))
                  (Utilities|Map|Add _pipelines_2 (.Pipeline (Utilities|Struct|BreakS_ArchitectSlot _array_element)) (Class|KismetMathLibrary|OrIntInt (.Value (Utilities|Map|Find _pipelines_2 (.Pipeline (Utilities|Struct|BreakS_ArchitectSlot _array_element)))) (Math|Conversions|ToInteger(Byte) (.Slot (Utilities|Struct|BreakS_ArchitectSlot _array_element)))))
                  (else
                    (Utilities|Map|Add _pipelines_3 (.Pipeline (Utilities|Struct|BreakS_ArchitectSlot _array_element)) (Math|Conversions|ToInteger(Byte) (.Slot (Utilities|Struct|BreakS_ArchitectSlot _array_element))))))))))
        (:then_1
          (if (> (Utilities|Map|Length (LocalVariables|Getpipelines)) 0)
            (bind _keys (Utilities|Map|Keys _pipelines))
            (bind _values_2 (Utilities|Map|Values _pipelines))
            (return false true _keys _values_2)
            (else
              (return false false 0 0))))))
    (:else
      (return false false 0 0))))

(fn FlipSplineDirection
  (|CallParentFunction)
  (PCG|Generate (Variables|Default|GetPCG_Main) true))

(fn SnapPointsZ
  (for _index (range 0 (- (Spline|GetNumberOfSplinePoints (Variables|Default|GetSpline)) 1))
    (Spline|SetLocationatSplinePoint (Variables|Default|GetSpline) _index (Math|Vector|MakeVector (.X (Math|Vector|BreakVector (.Position (Utilities|Struct|BreakSplinePoint (Spline|GetSplinePointAt (Variables|Default|GetSpline) _index "Local"))))) (.Y (Math|Vector|BreakVector (.Position (Utilities|Struct|BreakSplinePoint (Spline|GetSplinePointAt (Variables|Default|GetSpline) _index "Local"))))) 0.0) "Local" false))
  (Spline|UpdateSpline (Variables|Default|GetSpline)))

(fn Print
  (LocalVariables|SetNewLocalVar 0)
  (for _array_element (Actor|GetComponentsByClass "/Script/Engine.InstancedStaticMeshComponent")
    (LocalVariables|SetNewLocalVar (+ (Components|InstancedStaticMesh|GetInstanceCount _array_element) (LocalVariables|GetNewLocalVar))))
  (Development|PrintString (Utilities|String|Append (Utilities|GetDisplayName self) " Spawned Instance Count of " (Utilities|String|ToString(Integer) (LocalVariables|GetNewLocalVar)))))

(fn PopulateRecipes
  (switch int (Variables|PCGINTERNAL|GetAssetVersion)))