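; BuildingSpline_Grammar is a spline-based building actor that feeds recipe assets and user settings to a PCG component for procedural generation.
; Its construction script resolves wall, floor, corner, height and top/middle/bottom recipe options into GEN variables, flattens spline points, derives a GUID-suffixed asset name and flags recipe problems.
; Helpers regenerate PCG, snap points to footprint-width steps and count instances.
; BeginPlay enables shadows on dynamic mesh components.
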(event EventBeginPlay
  (|CallParentFunction)
  (PCGINTERNAL|ProcessDynFloorMeshs))

(event Collision|EventActorBeginOverlap
  (params (OtherActor :type Actor%20Object%20Reference))
  (|CallParentFunction OtherActor) ; This node is disabled and will not be called.\nDrag off pins to build functionality.
)

(event EventTick
  (params (DeltaSeconds :type Float%20%28single-precision%29))
  (|CallParentFunction DeltaSeconds) ; This node is disabled and will not be called.\nDrag off pins to build functionality.
)

(fn ConstructionScript
  (bind _footprint (Properties|GetFootprintSize))
  (bind _buildingoffset (Variables|00-Core|GetBuildingOffset))
  (bind _baserecipe (Variables|01-Recipes|GetBaseRecipe))
  (|CallParentFunction)
  (Utilities|FlowControl|Sequence
    (:then_0
      (Variables|01-Recipes|GetBaseRecipe
        (:then
          (Variables|PCGINTERNAL|SetGEN_Enabled_0 true)
          (Utilities|FlowControl|Sequence
            (:then_0
              ;[0.3628 0.3628 0.3628 0.5] Extract
              (Variables|PCGINTERNAL|SetGEN_FootprintSize (Math|Vector|SelectVector (* (.z (Transformation|GetActorScale3D)) _footprint) _footprint (Utilities|Enum|Equal(Enum) (Variables|00-Core|Editor|GetVerticalScalingBehavior) "NewEnumerator1"))))
            (:then_1
              (Variables|PCGINTERNAL|FeatureToggles|SetGEN_HasZStack (> (Variables|PCGINTERNAL|GetGEN_ZCount) 1)))
            (:then_2
              (Variables|PCGINTERNAL|SetGEN_ExportPath (Utilities|String|Append "/Game/" (Variables|03-Floors|GetProjectSavePath))))))
        (:else
          (Variables|PCGINTERNAL|SetGEN_Enabled_0 false))))
    (:then_1
      (CallFunction|GetUniqueID))
    (:then_2
      (PCGINTERNAL|PopulateRecipes))
    (:then_3
      (if (Variables|PCGINTERNAL|GetGEN_Enabled_0)
        (Utilities|FlowControl|Sequence
          (:then_0
            ;[0.3628 0.3628 0.3628 0.176] Extract High Level Booleans
            (Utilities|FlowControl|Sequence
              (:then_0
                ;;[0.3628 0.3628 0.3628 0.5] Walls
                (Variables|PCGINTERNAL|FeatureToggles|SetGEN_WallsEnabled (Variables|02-Walls|GetSpawnWalls)))
              (:then_1
                ;;[0.3628 0.3628 0.3628 0.5] Floors
                (Variables|PCGINTERNAL|FeatureToggles|SetGEN_FloorsEnabled (Variables|03-Floors|GetSpawnFloors))
                (Variables|PCGINTERNAL|FeatureToggles|SetGEN_CeilingEnabled (Variables|03-Floors|GetSpawnCeiling)))
              (:then_2
                ;;[0.125 0.125 0.125 0.5] Corners
                (Utilities|FlowControl|Sequence
                  (:then_0
                    (bind _output_get (Variables|PCGINTERNAL|SetGEN_InCornerMode_Walls (select (Variables|02-Walls|Corners|GetDisableCornersIn) "NewEnumerator0" (Variables|/ArchitectCore/Core/ArchitectAssets/ArchitectFullRecipe.ArchitectFullRecipe_C|GetInvertedCornerMode _baserecipe))))
                    (bind _output_get_2 (Variables|PCGINTERNAL|SetGEN_OutCornerMode_Walls (select (Variables|02-Walls|Corners|GetDisableCornersOut) "NewEnumerator0" (Variables|/ArchitectCore/Core/ArchitectAssets/ArchitectFullRecipe.ArchitectFullRecipe_C|GetOutsideCornerMode _baserecipe))))
                    (Variables|PCGINTERNAL|FeatureToggles|SetGEN_CornersEnabled (not (and (Utilities|Enum|Equal(Enum) _output_get "NewEnumerator0") (Utilities|Enum|Equal(Enum) _output_get_2 "NewEnumerator0")))))))
              (:then_3
                ;[0.3628 0.3628 0.3628 0.5] May do some processing on floors, to remove duplicates or clamp to bounds
                (Variables|PCGINTERNAL|SetGEN_SpawnGroundFloor (Variables|03-Floors|GetSpawnGroundFloor))
                (bind _output_get_3 (Variables|PCGINTERNAL|FeatureToggles|SetGEN_MultifloorEnabled (Variables|03-Floors|Multifloor|GetEnableMultifloor)))
                (if _output_get_3
                  (Variables|PCGINTERNAL|SetGEN_MultiFloors (Variables|03-Floors|Multifloor|GetMulti%20Floors))
                  (Variables|PCGINTERNAL|FeatureToggles|SetGEN_MultifloorEnabled (Variables|03-Floors|Multifloor|GetEnableMultifloor))))))
          (:then_1
            ;[0.15 0.15 0.15 0.5] Set Building Height
            (Variables|PCGINTERNAL|SetGEN_BuildingHeight (Variables|00-Core|GetBuilding%20Height))
            (Variables|PCGINTERNAL|SetGEN_Footprint (Properties|GetFootprintSize)))
          (:then_3
            ;[1 1 1] Top Bottom Recipes
            (Utilities|FlowControl|Sequence
              (:then_0
                (Variables|01-Recipes|OverrideRecipes|GetTopRecipe
                  (:then
                    (Variables|PCGINTERNAL|FeatureToggles|SetGEN_OverrideTop (Variables|01-Recipes|OverrideRecipes|GetEnableTopRecipe)))
                  (:else
                    (Variables|PCGINTERNAL|FeatureToggles|SetGEN_OverrideTop false))))
              (:then_1
                (Variables|01-Recipes|OverrideRecipes|GetBottomRecipe
                  (:then
                    (Variables|PCGINTERNAL|FeatureToggles|SetGEN_OverrideBottom (Variables|01-Recipes|OverrideRecipes|GetEnableBottomRecipe)))
                  (:else
                    (Variables|PCGINTERNAL|FeatureToggles|SetGEN_OverrideBottom false))))
              (:then_2
                (Variables|PCGINTERNAL|Recipes|SetGEN_MiddleRecipe (Variables|01-Recipes|GetBaseRecipe))
                (Variables|PCGINTERNAL|Recipes|SetGEN_BottomRecipe (select (Variables|PCGINTERNAL|FeatureToggles|GetGEN_OverrideBottom) (Variables|01-Recipes|OverrideRecipes|GetBottomRecipe) (Variables|01-Recipes|GetBaseRecipe)))
                (Variables|PCGINTERNAL|Recipes|SetGEN_TopRecipe (select (Variables|PCGINTERNAL|FeatureToggles|GetGEN_OverrideTop) (Variables|01-Recipes|OverrideRecipes|GetTopRecipe) (Variables|01-Recipes|GetBaseRecipe))))))
          (:then_4
            (CallFunction|SnapPointsZ))
          (:then_5
            ;[1 1 1] Calculate Absolute Offset
            (bind _output_get_4 (Variables|PCGINTERNAL|SetGEN_BuildingOffset (* (Math|Transform|TransformDirection (Transformation|GetActorTransform) (Math|Vector|Normalize _buildingoffset)) (Math|Vector|VectorLength _buildingoffset))))
            (Variables|PCGINTERNAL|SetGEN_HasBuildingOffset (Utilities|Operators|NotEqual(!=) :A _output_get_4)))
          (:then_6
            ;[1 1 1] DEPRICATED Pipelines
            (Variables|PCGINTERNAL|SetGEN_UseInstanceOverride false)
            (Variables|PCGINTERNAL|SetGEN_HasAssetOverrides false)
            (Variables|PCGINTERNAL|SetGEN_HasPipelineOverrides false)))))
    (:then_4
      ;[0.6233 0.5277 0 0.5] Check for Warnigns
      (CallFunction|CheckforWarnings (Variables|01-Recipes|GetBaseRecipe))
      (Utilities|FlowControl|Sequence
        (:then_0
          (if (Variables|01-Recipes|OverrideRecipes|GetEnableTopRecipe)
            (CallFunction|CheckforWarnings (Variables|01-Recipes|OverrideRecipes|GetTopRecipe))))
        (:then_1
          (if (Variables|01-Recipes|OverrideRecipes|GetEnableBottomRecipe)
            (CallFunction|CheckforWarnings (Variables|01-Recipes|OverrideRecipes|GetBottomRecipe))))))))

(fn GetBoundsVerticalHeight
  (return (Math|Float|Max(Float) (.Z (Math|Vector|BreakVector (Properties|GetFootprintSize))) (Variables|00-Core|GetBuilding%20Height))))

(fn GetFootprintSize
  (bind _baserecipe (Variables|01-Recipes|GetBaseRecipe)
    (:then
      (if (> (Math|Vector|VectorLength (Variables|/ArchitectCore/Core/ArchitectAssets/ArchitectFullRecipe.ArchitectFullRecipe_C|GetFootprint _baserecipe)) 3.0)
        _
        (else
          (CallFunction|PrintErrorwithInfo "Given Recipe with very small footprint, make this larger or it could spawn a huge number of objects" true)))
      (return (* (Variables|00-Core|GetFootprintScaleMultiplier) (Variables|/ArchitectCore/Core/ArchitectAssets/ArchitectFullRecipe.ArchitectFullRecipe_C|GetFootprint _baserecipe))))
    (:else
      (CallFunction|PrintErrorwithInfo "Missing Base Recipe" false)
      (return "50.000000,50.000000,50.000000"))))

(fn RefreshGeneration
  (Class|PCGComponent|GenerateLocal (Variables|Default|GetPCG_Main) true))

(fn SearchforOverrides
  (bind _baserecipe (Variables|01-Recipes|GetBaseRecipe))
  (bind _pipelines (LocalVariables|Getpipelines))
  (bind _pipelines_2 (LocalVariables|Getpipelines))
  (Variables|01-Recipes|GetBaseRecipe
    (:then
      (Utilities|FlowControl|Sequence
        (:then_0
          (bind _slot_lookups (Default|GetSlotsasLookup _baserecipe))
          (bind _values (Utilities|Map|Values _slot_lookups))
          (for _array_element _values
            (if (.Enabled (Utilities|Struct|BreakS_ArchitectSlot _array_element))
              (if (!= (.Pipeline (Utilities|Struct|BreakS_ArchitectSlot _array_element)) (Variables|/ArchitectCore/Core/ArchitectAssets/ArchitectFullRecipe.ArchitectFullRecipe_C|GetDefaultPipeline _baserecipe))
                (if (Utilities|Map|Contains _pipelines_2 (.Pipeline (Utilities|Struct|BreakS_ArchitectSlot _array_element)))
                  (Utilities|Map|Add _pipelines (.Pipeline (Utilities|Struct|BreakS_ArchitectSlot _array_element)) (Class|KismetMathLibrary|OrIntInt (.Value (Utilities|Map|Find _pipelines (.Pipeline (Utilities|Struct|BreakS_ArchitectSlot _array_element)))) (Math|Conversions|ToInteger(Byte) (.Slot (Utilities|Struct|BreakS_ArchitectSlot _array_element)))))
                  (else
                    (Utilities|Map|Add _pipelines_2 (.Pipeline (Utilities|Struct|BreakS_ArchitectSlot _array_element)) (Math|Conversions|ToInteger(Byte) (.Slot (Utilities|Struct|BreakS_ArchitectSlot _array_element))))))))))))
    (:else
      (return false false 0 0))))

(fn SnapPointsZ
  (for _index (range 0 (- (Spline|GetNumberOfSplinePoints (Variables|Default|GetSpline)) 1))
    (Spline|SetLocationatSplinePoint (Variables|Default|GetSpline) _index (Math|Vector|MakeVector (.X (Math|Vector|BreakVector (.Position (Utilities|Struct|BreakSplinePoint (Spline|GetSplinePointAt (Variables|Default|GetSpline) _index "Local"))))) (.Y (Math|Vector|BreakVector (.Position (Utilities|Struct|BreakSplinePoint (Spline|GetSplinePointAt (Variables|Default|GetSpline) _index "Local"))))) 0.0) "Local" false))
  (Spline|UpdateSpline (Variables|Default|GetSpline)))

(fn PrintInstanceCount
  (LocalVariables|SetNewLocalVar 0)
  (for _array_element (Actor|GetComponentsByClass "/Script/Engine.InstancedStaticMeshComponent")
    (LocalVariables|SetNewLocalVar (+ (Components|InstancedStaticMesh|GetInstanceCount _array_element) (LocalVariables|GetNewLocalVar))))
  (Development|PrintString (Utilities|String|Append (Utilities|GetDisplayName self) " Spawned Instance Count of " (Utilities|String|ToString(Integer) (LocalVariables|GetNewLocalVar)))))

(fn ProcessDynFloorMeshs
  (for _array_element (Actor|GetComponentsByClass "/Script/GeometryFramework.DynamicMeshComponent")
    (Class|BaseDynamicMeshComponent|SetShadowsEnabled _array_element true)))

(fn PopulateRecipes
  (Utilities|Array|Clear (Variables|PCGINTERNAL|Recipes|GetGEN_AllRecipes))
  (Utilities|FlowControl|Sequence
    (:then_0
      (Utilities|Array|AddUnique (Variables|PCGINTERNAL|Recipes|GetGEN_AllRecipes) (Variables|PCGINTERNAL|Recipes|GetGEN_TopRecipe)))
    (:then_1
      (Utilities|Array|AddUnique (Variables|PCGINTERNAL|Recipes|GetGEN_AllRecipes) (Variables|PCGINTERNAL|Recipes|GetGEN_MiddleRecipe)))
    (:then_2
      (Utilities|Array|AddUnique (Variables|PCGINTERNAL|Recipes|GetGEN_AllRecipes) (Variables|PCGINTERNAL|Recipes|GetGEN_BottomRecipe)))))

(fn SnapSplinePoints
  (LocalVariables|Setx (.X (Math|Vector|BreakVector (Properties|GetFootprintSize))))
  (for _index (range 1 (- (Spline|GetNumberOfSplinePoints (Variables|Default|GetSpline)) 1))
    (LocalVariables|SetcurIndex _index)
    (Spline|SetLocationatSplinePoint (Variables|Default|GetSpline) (LocalVariables|GetcurIndex) (+ (Spline|GetLocationatSplinePoint (Variables|Default|GetSpline) (- (LocalVariables|GetcurIndex) 1) "Local") (* (Math|Vector|Normalize (- (Spline|GetLocationatSplinePoint (Variables|Default|GetSpline) (LocalVariables|GetcurIndex) "Local") (Spline|GetLocationatSplinePoint (Variables|Default|GetSpline) (- (LocalVariables|GetcurIndex) 1) "Local"))) (* (LocalVariables|Getx) (Math|Float|Round (/ (Math|Vector|Distance(Vector) (Spline|GetLocationatSplinePoint (Variables|Default|GetSpline) (LocalVariables|GetcurIndex) "Local") (Spline|GetLocationatSplinePoint (Variables|Default|GetSpline) (- (LocalVariables|GetcurIndex) 1) "Local")) (LocalVariables|Getx)))))) "Local" false))
  (Spline|UpdateSpline (Variables|Default|GetSpline)))

(fn CheckforWarnings
  (params (Target :type Architect%20Full%20Recipe%20Object%20Reference))
  (bind _slot_lookups (Default|GetSlotsasLookup Target))
  (bind _values (Utilities|Map|Values _slot_lookups))
  (for _array_element _values
    (if (.Enabled (Utilities|Struct|BreakS_ArchitectSlot _array_element))
      (if (.IsWall (Utilities|Struct|BreakS_ArchitectSlot _array_element))
        (if (or (!= (.Yaw (Math|Rotator|BreakRotator (.Rotation (Utilities|Struct|BreakArchitectAsset_TransformOptions (.TransformOptions (Utilities|Struct|BreakArchitectAsset (.DefaultAssets (Utilities|Struct|BreakS_ArchitectSlot _array_element)))))))) 0.0) (!= (.Yaw (Math|Rotator|BreakRotator (.Rotation (Utilities|Struct|BreakArchitectAsset_TransformOptions (.TransformOptions (Utilities|Struct|BreakArchitectAsset (.DefaultAssets (Utilities|Struct|BreakS_ArchitectSlot _array_element)))))))) 1.8e+02))
          (Development|PrintText (Utilities|Text|FormatText "RECIPE WARNING: Recipe {1} - Rotation of slot {0} is non 0 value, walls may not be scaled correctly " (Utilities|GetDisplayName Target) (Utilities|String|EnumtoString (.Slot (Utilities|Struct|BreakS_ArchitectSlot _array_element)))) true true "(R=1.000000,G=0.859050,B=0.000000,A=1.000000)"))))))

(fn GetUniqueID
  (bind _guids (LocalVariables|Getguids))
  (bind _returnvalue (Utilities|Set|Length _guids))
  (Utilities|FlowControl|Sequence
    (:then_0
      (if (Variables|03-Floors|GetUseDisplayNameAsAssetName)
        (Variables|03-Floors|SetAssetName (Utilities|String|StringToName (Utilities|GetDisplayName self)))))
    (:then_1
      (bind _outactors (Actor|GetAllActorsOfClass "BuildingSpline_Grammar_C"))
      (for _array_element _outactors
        (if (not (== _array_element self))
          (if (== (Variables|BuildingSpline_Grammar_C|GetAssetName _array_element) (Variables|03-Floors|GetAssetName))
            (if (!= (Variables|BuildingSpline_Grammar_C|GetGUID _array_element) -1)
              (Utilities|Set|Add (LocalVariables|Getguids) (Variables|BuildingSpline_Grammar_C|GetGUID _array_element))))))
      (if (> _returnvalue 0)
        (bind _index (Utilities|FlowControl|ForLoopwithBreak 0 (- _returnvalue _returnvalue) :!label _label)
          (:LoopBody
            (if (not (Utilities|Set|Contains _guids _index))
              (Variables|03-Floors|SetGUID _index)
              (LocalVariables|Setfound true)
              (goto _label Break)))
          (:Completed
            (if (not (LocalVariables|Getfound))
              (Variables|03-Floors|SetGUID _returnvalue))))
        (else
          (Variables|03-Floors|SetGUID 0))))
    (:then_2
      (Variables|03-Floors|SetGEN_AssetName (Utilities|String|StringToName (Utilities|String|Append (Utilities|String|ToString(Name) (Variables|03-Floors|GetAssetName)) (Utilities|String|ToString(Integer) (Variables|03-Floors|GetGUID))))))))