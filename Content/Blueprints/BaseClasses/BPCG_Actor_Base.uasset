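; Base actor for PCG-driven Blueprints that sizes the bounding box used for procedural generation.
; The Construction Script sets a force-downscale flag from DesignerMode, then centers and resizes PCGBoundingBox around padded bounds, skipping near-zero XY spans.
; GetBoundsMinMax returns zero here, apparently as an override point for child classes, alongside an empty PreConstruct hook.
; Graph assignment is disconnected, and the error-print helper does not use its message.
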(event EventBeginPlay)

(event Collision|EventActorBeginOverlap
  (params (OtherActor :type Actor%20Object%20Reference)))

(event EventTick
  (params (DeltaSeconds :type Float%20%28single-precision%29)))

(fn ConstructionScript
  (Utilities|FlowControl|Sequence
    (:then_0
      (Variables|PCGINTERNAL|SetGEN_ForceDownscale (EditorOnly|IsForceDownscaleEnabled)))
    (:then_2
      (Bounds|UpdateBoundsforPCG))))

(fn PreConstruct)

(fn UpdateBoundsforPCG
  (bind _boundspadding (Variables|00-Core|GetBoundsPadding))
  (bind (_min _max) (Bounds|GetBoundsMinMax))
  (bind _output_get (LocalVariables|SetMin _min))
  (bind _output_get_2 (LocalVariables|SetMax _max))
  (if (not (<= (Class|KismetMathLibrary|VectorDistance2DSquared _output_get_2 _output_get) 0.1))
    (Transformation|SetRelativeLocation (Variables|Default|GetPCGBoundingBox) (Math|Vector|Lerp(Vector) (+ (LocalVariables|GetMax) _boundspadding) (- (LocalVariables|GetMin) _boundspadding) 0.5) false false)
    (Components|Box|SetBoxExtent (Variables|Default|GetPCGBoundingBox) (Math|Vector|VectorGetAbs (/ (- (+ (LocalVariables|GetMax) _boundspadding) (- (LocalVariables|GetMin) _boundspadding)) 2.0)) true)))

(fn GetBoundsMinMax
  (return "0, 0, 0" "0, 0, 0"))

(fn PrintErrorwithInfo
  (params (Error%20Message :type String) (bPrintToScreen :type Boolean))
  (Development|PrintString "Hello" bPrintToScreen true "(R=1.000000,G=0.113641,B=0.000000,A=1.000000)"))

(fn IsForceDownscaleEnabled
  (return (Variables|00-Core|GetDesignerMode)))