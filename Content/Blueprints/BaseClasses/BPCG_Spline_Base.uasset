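; Base actor Blueprint for spline-driven tools, apparently PCG by its name, whose construction script applies the IsClosedLoop setting to its Spline.
; GetBoundsMinMax builds local bounds from splines with over two points, raising the maximum by GetBoundsVerticalHeight, which returns zero here.
; FlipSplineDirection reverses point order by rewriting positions only, without copying tangents or rotations, then updates the spline.
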(event EventBeginPlay
  (|CallParentFunction) ; This node is disabled and will not be called.\nDrag off pins to build functionality.
)

(event Collision|EventActorBeginOverlap
  (params (OtherActor :type Actor%20Object%20Reference))
  (|CallParentFunction OtherActor) ; This node is disabled and will not be called.\nDrag off pins to build functionality.
)

(event EventTick
  (params (DeltaSeconds :type Float%20%28single-precision%29))
  (|CallParentFunction DeltaSeconds) ; This node is disabled and will not be called.\nDrag off pins to build functionality.
)

(fn ConstructionScript
  (|CallParentFunction)
  (Utilities|FlowControl|Sequence
    (:then_0
      (Spline|SetClosedLoop (Variables|Default|GetSpline) (Variables|00-Core|GetIsClosedLoop) true))))

(fn GetBoundsMinMax
  (bind _spline (Variables|Default|GetSpline))
  (bind _spline_2 (Variables|Default|GetSpline))
  (bind _returnvalue (Spline|GetNumberOfSplinePoints _spline))
  (bind _returnvalue_2 (Spline|GetLocationatSplinePoint _spline_2 0 "Local"))
  (LocalVariables|Setoffset (Math|Vector|MakeVector 0.0 0.0 (Bounds|GetBoundsVerticalHeight)))
  (LocalVariables|Setminimum _returnvalue_2)
  (LocalVariables|Setmaximum (+ _returnvalue_2 (LocalVariables|Getoffset)))
  (if (> _returnvalue 2)
    (for _index (range 1 (- _returnvalue 1))
      (LocalVariables|Setminimum (Math|Vector|MakeVector (Math|Float|Min(Float) (.X (Math|Vector|BreakVector (Spline|GetLocationatSplinePoint (Variables|Default|GetSpline) _index "Local"))) (.X (Math|Vector|BreakVector (LocalVariables|Getminimum)))) (Math|Float|Min(Float) (.Y (Math|Vector|BreakVector (Spline|GetLocationatSplinePoint (Variables|Default|GetSpline) _index "Local"))) (.Y (Math|Vector|BreakVector (LocalVariables|Getminimum)))) (Math|Float|Min(Float) (.Z (Math|Vector|BreakVector (Spline|GetLocationatSplinePoint (Variables|Default|GetSpline) _index "Local"))) (.Z (Math|Vector|BreakVector (LocalVariables|Getminimum))))))
      (LocalVariables|Setmaximum (Math|Vector|MakeVector (Math|Float|Max(Float) (.x (+ (Spline|GetLocationatSplinePoint (Variables|Default|GetSpline) _index "Local") (LocalVariables|Getoffset))) (.X (Math|Vector|BreakVector (LocalVariables|Getmaximum)))) (Math|Float|Max(Float) (.y (+ (Spline|GetLocationatSplinePoint (Variables|Default|GetSpline) _index "Local") (LocalVariables|Getoffset))) (.Y (Math|Vector|BreakVector (LocalVariables|Getmaximum)))) (Math|Float|Max(Float) (.z (+ (Spline|GetLocationatSplinePoint (Variables|Default|GetSpline) _index "Local") (LocalVariables|Getoffset))) (.Z (Math|Vector|BreakVector (LocalVariables|Getmaximum)))))))
    (return (LocalVariables|Getminimum) (LocalVariables|Getmaximum))))

(fn GetBoundsVerticalHeight
  (return 0.0))

(fn FlipSplineDirection
  (bind _spline (Variables|Default|GetSpline))
  (bind _returnvalue (Spline|GetNumberOfSplinePoints _spline))
  (bind _returnvalue_2 (- _returnvalue 1))
  (LocalVariables|Setlen _returnvalue_2)
  (for _index (range 0 _returnvalue_2)
    (Utilities|Array|SetArrayElem (LocalVariables|Getnew%20points) (- (LocalVariables|Getlen) _index) (Spline|GetSplinePointAt (Variables|Default|GetSpline) _index "Local") true))
  (for (_array_element _array_index) (LocalVariables|Getnew%20points)
    (Spline|SetLocationatSplinePoint (Variables|Default|GetSpline) _array_index (.Position (Utilities|Struct|BreakSplinePoint _array_element)) "Local" false))
  (Spline|UpdateSpline (Variables|Default|GetSpline)))