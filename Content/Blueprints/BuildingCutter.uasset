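; BuildingCutter is a placeable volume actor that marks where PCG effects erase or cut doors, windows or custom openings in buildings.
; Its construction script tints the Cube gizmo per Mode through a dynamic material instance.
; It then replaces the actor's tags with one built from Mode, prefixed Wall_ or Floor_ unless both are affected, so PCG can group effects.
; All runtime events are empty.
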(event EventBeginPlay)

(event Collision|EventActorBeginOverlap
  (params (OtherActor :type Actor%20Object%20Reference)))

(event EventTick
  (params (DeltaSeconds :type Float%20%28single-precision%29)))

(fn ConstructionScript
  (bind _mode (Variables|Default|GetMode))
  (bind _affectwalls (Variables|Default|GetAffectWalls))
  (bind _tags (Variables|Default|GetTags))
  (bind _cube (Variables|Default|GetCube))
  (bind _returnvalue (Utilities|Select :Index _mode :NewEnumerator0 "Eraser" :NewEnumerator1 "Door" :NewEnumerator2 "Window" :NewEnumerator3 "Custom"))
  (Utilities|FlowControl|Sequence
    (:then_0
      ;[0.06051 0.276 0] Gizmos
      (bind _returnvalue_2 (Rendering|Material|CreateDynamicMaterialInstance _cube 0 (Rendering|Material|GetMaterial _cube 0) "None" :!class /Script/Engine.PrimitiveComponent))
      (Rendering|Material|SetVectorParameterValue _returnvalue_2 "Color" (Utilities|Select :Index (Variables|Default|GetMode) :NewEnumerator0 "(R=1.000000,G=0.247059,B=0.929412,A=1.000000)" :NewEnumerator1 "(R=0.125490,G=1.000000,B=0.000000,A=1.000000)" :NewEnumerator2 "(R=0.000000,G=1.000000,B=0.949020,A=1.000000)" :NewEnumerator3 "(R=1.000000,G=0.000000,B=0.009486,A=1.000000)") :!class /Script/Engine.MaterialInstanceDynamic))
    (:then_1
      (Utilities|Array|Add (LocalVariables|Gettmp) (Utilities|String|StringToName (Utilities|String|SelectString _returnvalue (Utilities|String|Append (Utilities|String|SelectString "Wall_" "Floor_" _affectwalls) _returnvalue) (and (Variables|Default|GetAffectFloors) _affectwalls)))))
    (:then_2
      ;[0.2459 0.1087 0.2604] Apply Tags to group PCG effects
      (Utilities|Array|Clear _tags)
      (for _array_element (LocalVariables|Gettmp)
        (Utilities|Array|Add _tags _array_element)))))

(fn UpdateTag
  (params (HasTag :type Boolean) (TagName :type Name))
  (if HasTag
    (Utilities|Array|AddUnique (Variables|Default|GetTags) TagName)
    (else
      (Utilities|Array|RemoveItem (Variables|Default|GetTags) TagName))))